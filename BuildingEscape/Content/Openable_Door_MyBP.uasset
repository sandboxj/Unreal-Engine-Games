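; Openable door actor that swings open and closed in response to the FDoorEvent interface's open and close calls.
; It stores its starting rotation on BeginPlay, and a DoorSwing timeline adds a yaw angle to that rotation as it plays.
; Closing reverses the same timeline, and a timeline event track plays a door lock sound at the door's location.
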(event OnClose(FDoorEvent)
  (bind _doorangle (Timeline|DoorSwing Reverse)
    (:Update
      (Transformation|SetActorRotation (Math|Rotator|CombineRotators (Math|Rotator|MakeRotator 0.0 0.0 _doorangle) (Variables|Default|GetInitialRotation))))
    (:SoundTiming
      (Audio|PlaySoundatLocation "/Game/Audio/door-lock.door-lock" (Transformation|GetActorLocation) "0, 0, 0" 0.5))))

(event OnOpen(FDoorEvent)
  (bind _doorangle (Timeline|DoorSwing Play)
    (:Update
      (Transformation|SetActorRotation (Math|Rotator|CombineRotators (Math|Rotator|MakeRotator 0.0 0.0 _doorangle) (Variables|Default|GetInitialRotation))))
    (:SoundTiming
      (Audio|PlaySoundatLocation "/Game/Audio/door-lock.door-lock" (Transformation|GetActorLocation) "0, 0, 0" 0.5))))

(event EventBeginPlay
  (Variables|Default|SetInitialRotation (Transformation|GetActorRotation)))

(fn ConstructionScript)